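; BP_Cube is a cube actor Blueprint that derives its world position from its own scale in the construction script.
; X and Y location come from the X and Y variables multiplied by the actor's Y scale and ScaleRatioY.
; Z location is the Z scale multiplied by ScaleRatioZ, so the actor is repositioned whenever construction reruns.
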(fn `UserConstructionScript`
  (bind _scaleratioy (`self.ScaleRatioY`))
  (bind _y (.y (`self.GetActorScale3D`)))
  (`self.K2_SetActorLocation` (`KismetMathLibrary.MakeVector` (* (* _y (`self.x`)) _scaleratioy) (* (* _y (`self.y`)) _scaleratioy) (* (.z (`self.GetActorScale3D`)) (`self.ScaleRatioZ`)))))