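; BP_PickupComponent lets its owning actor be picked up and dropped, with BP_MotionController calling Pickup.
; BeginPlay caches the owner's static mesh components, and Pickup disables their physics while Drop re-enables it.
; Instead of attaching, a Tick gate opened by Pickup and closed by Drop moves the owner to the given scene component's location with sweep and teleport, leaving rotation untouched.
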(event `self.ReceiveBeginPlay`
  (set `self.TargetStaticMesh` (`Actor.K2_GetComponentsByClass` (`self.GetOwner`) "/Script/Engine.StaticMeshComponent")))

(event `self.ReceiveTick`
  (params (DeltaSeconds :type "Float (single-precision)"))
  (bind _rootscene (`self.RootScene`))
  (`/Engine/EditorBlueprintResources/StandardMacros.Gate` true :!label _label
    (:`Exit`
      (`/Engine/EditorBlueprintResources/StandardMacros.IsValid` _rootscene
        (:`Is Valid`
          (`Actor.K2_SetActorLocation` (`self.GetOwner`) (`self.K2_GetComponentLocation` _rootscene) true true))))))

(event `/Game/VirtualRealityBP/Blueprints/PickupActorInterface.Pickup`
  (params (AttachTo :type "SceneComponent Object Reference"))
  (set `self.RootScene` AttachTo)
  (for _array_element (`self.TargetStaticMesh`)
    (`PrimitiveComponent.SetSimulatePhysics` _array_element false))
  (goto _label :!via `Open`))

(event `/Game/VirtualRealityBP/Blueprints/PickupActorInterface.Drop`
  (for _array_element (`self.TargetStaticMesh`)
    (`PrimitiveComponent.SetSimulatePhysics` _array_element true))
  (goto _label :!via `Close`))