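; BP_TracingUnit is an AI character that is lured toward the most important perceived target.
; Perception updates filter actors by class, keeping the highest BP_BePersetibleComponent priority, with distance breaking ties.
; When nearly stationary with that target sighted and in range, Tick starts SimpleMoveToActor and opens a gate that halts movement once the target exceeds perception distance.
; The construction script positions a perception display cone.
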(event `self.AIPerception.OnPerceptionUpdated`
  (params (UpdatedActors :type "Array of Actor Object Reference"))
  (bind _mostpriority (`self.MostPriority`))
  ;[1 1 1] Update Perception Target
  (for _array_element UpdatedActors
    (if (`KismetArrayLibrary.Array_Contains` (`self.TargetActorArray`) (`GameplayStatics.GetObjectClass` _array_element))
      (bind _returnvalue (`self.GetComponentByClass` _array_element "/Game/BP_BePersetibleComponent.BP_BePersetibleComponent_C"))
      (`/Engine/EditorBlueprintResources/StandardMacros.IsValid` _returnvalue
        (:`Is Valid`
          (bind _priority (`/Game/BP_BePersetibleComponent.Priority` _returnvalue))
          (if (> _priority _mostpriority)
            (set `self.NearestPriorityTarget` _array_element)
            (set `self.NearestPriorityDistance` (`self.GetDistanceTo` _array_element))
            (set `self.MostPriority` _priority)
            (elif (== _priority _mostpriority)
              (bind _returnvalue_2 (`self.GetDistanceTo` _array_element))
              (if (< _returnvalue_2 (`self.NearestPriorityDistance`))
                (set `self.NearestPriorityTarget` _array_element)
                (set `self.NearestPriorityDistance` _returnvalue_2)))))))))

(event `self.ReceiveTick`
  (params (DeltaSeconds :type "Float (single-precision)"))
  (bind _nearestprioritytarget (`self.NearestPriorityTarget`))
  ;[1 1 1] be Lured to Target
  (`|ExecutionSequence`
    (:`then_0`
      (`/Engine/EditorBlueprintResources/StandardMacros.Gate` true :!label _label
        (:`Exit`
          (if (> (`self.GetDistanceTo` (`self.NearestPriorityTarget`)) (`self.PerceptionDistance`))
            (`self.StopTrace`)
            (goto _label :!via `Close`)))))
    (:`then_1`
      (if (`KismetMathLibrary.NearlyEqual_FloatFloat` (`KismetMathLibrary.VSizeSquared` (`MovementComponent.Velocity` (`self.CharacterMovement`))) 0.0 0.1)
        (if (`KismetArrayLibrary.Array_Contains` (`AIPerceptionComponent.GetCurrentlyPerceivedActors` (`self.AIPerception`) "/Script/AIModule.AISense_Sight") _nearestprioritytarget)
          (if (<= (`self.GetDistanceTo` _nearestprioritytarget) (`self.PerceptionDistance`))
            (`self.StartTrace`)
            (goto _label :!via `Open`)))))))

(fn `StartTrace`
  (`NavigationSystem.SimpleMoveToActor` (`self.GetController`) (`self.NearestPriorityTarget`)))

(fn `StopTrace`
  (`MovementComponent.StopMovementImmediately` (`self.CharacterMovement`)))

(fn `UserConstructionScript`
  (`SceneComponent.K2_SetRelativeLocation` (`self.PerceptionDisplayCone`) (`KismetMathLibrary.MakeVector` (- (* (* (`self.PerceptionVolumePositionRatio`) (.x (`SceneComponent.K2_GetComponentScale` (`self.PerceptionDisplayCone`)))) 1.75) 10.0) 1.0 (* (`CapsuleComponent.GetScaledCapsuleHalfHeight` (`self.CapsuleComponent`)) 0.5)) false false))