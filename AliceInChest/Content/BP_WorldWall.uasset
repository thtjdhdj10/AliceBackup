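; BP_WorldWall is a wall actor that sizes and places itself relative to a referenced floor actor.
; Its construction script derives wall length from the floor's X scale, keeping thickness and height fixed.
; It then sets its location from that length times the X and Y factors and ScaleRatioY, with Z from height times ScaleRatioZ, so the offset is measured from the world origin.
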(fn `UserConstructionScript`
  (bind _scaleratioy (`self.ScaleRatioY`))
  (bind _y (.y (`self.GetActorScale3D`)))
  (`self.SetActorScale3D` (`KismetMathLibrary.MakeVector` 0.2 (* (.x (`self.GetActorScale3D` (`self.FloorActor`))) 40.0) 6.0))
  (`self.K2_SetActorLocation` (`KismetMathLibrary.MakeVector` (* (* _y (`self.x`)) _scaleratioy) (* (* _y (`self.y`)) _scaleratioy) (* (.z (`self.GetActorScale3D`)) (* (`self.ScaleRatioZ`) 1.0)))))