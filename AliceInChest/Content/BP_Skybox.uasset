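; BP_Skybox is one plane face of a sunny skybox, with Direction selecting left, right, front, back or top.
; The construction script picks that face's rotation, axis offset and Sunny_01A material.
; It then overwrites the actor transform, positioning the face relative to world origin from RoomScale and scaling it by ScaleRatio and ScaleZ.
; Side offsets also depend on current actor scale, while the top face uses its own height formula.
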(fn `UserConstructionScript`
  (bind _roomscale (`self.RoomScale`))
  (bind _rotation (`self.Rotation`))
  (bind _scaleratio (`self.ScaleRatio`))
  (bind _plane (`self.Plane`))
  (bind _y (.y (`self.GetActorScale3D`)))
  (bind _returnvalue (* _scaleratio 1.0))
  (bind _returnvalue_2 (`KismetMathLibrary.MakeVector` _returnvalue _returnvalue (* (`self.ScaleZ`) 1.0)))
  (bind _returnvalue_3 (* (* _y (`self.x`)) _roomscale))
  (bind _returnvalue_4 (* (* _y (`self.y`)) _roomscale))
  (switch `/Game/Skybox/SkyboxDirection` (`self.Direction`)
    (:`NewEnumerator1`
      (set `self.Rotation` (struct :`Yaw` 90.0 :`Roll` -90.0))
      (set `self.x` 0.0)
      (set `self.y` -1.0)
      (`PrimitiveComponent.SetMaterial` _plane 0 "/Game/Skybox/Sunny_01A_left_Mat.Sunny_01A_left_Mat")
      (`self.K2_SetActorTransform` (`KismetMathLibrary.MakeTransform` (`KismetMathLibrary.MakeVector` _returnvalue_3 _returnvalue_4 (* (.z (`self.GetActorScale3D`)) _roomscale)) _rotation _returnvalue_2) :!label _label))
    (:`NewEnumerator2`
      (set `self.Rotation` (struct :`Yaw` -180.0 :`Roll` 90.0))
      (set `self.x` 0.0)
      (set `self.y` 1.0)
      (`PrimitiveComponent.SetMaterial` _plane 0 "/Game/Skybox/Sunny_01A_right_Mat.Sunny_01A_right_Mat")
      (goto _label))
    (:`NewEnumerator3`
      (set `self.Rotation` (struct :`Yaw` 90.0 :`Roll` 90.0))
      (set `self.x` 1.0)
      (set `self.y` 0.0)
      (`PrimitiveComponent.SetMaterial` _plane 0 "/Game/Skybox/Sunny_01A_front_Mat.Sunny_01A_front_Mat")
      (goto _label))
    (:`NewEnumerator4`
      (set `self.Rotation` (struct :`Yaw` 90.0 :`Roll` 90.0))
      (set `self.x` -1.0)
      (set `self.y` 0.0)
      (`PrimitiveComponent.SetMaterial` _plane 0 "/Game/Skybox/Sunny_01A_back_Mat.Sunny_01A_back_Mat")
      (goto _label))
    (:`NewEnumerator5`
      (set `self.Rotation` (struct :`Yaw` 90.0 :`Roll` 180.0))
      (set `self.x` 0.0)
      (set `self.y` 0.0)
      (`PrimitiveComponent.SetMaterial` _plane 0 "/Game/Skybox/Sunny_01A_up_Mat.Sunny_01A_up_Mat")
      (`self.K2_SetActorTransform` (`KismetMathLibrary.MakeTransform` (`KismetMathLibrary.MakeVector` _returnvalue_3 _returnvalue_4 (* (* _roomscale 2.0) _scaleratio)) _rotation _returnvalue_2)))))