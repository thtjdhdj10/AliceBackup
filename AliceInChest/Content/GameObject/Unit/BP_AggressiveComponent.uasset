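; BP_AggressiveComponent is an actor component that detects when its owning BP_TracingUnit overlaps one of its target actor types.
; On BeginPlay it copies the owner's TargetActorArray, destroying itself if the owner is not a BP_TracingUnit.
; Every Tick it polls the owner's overlapping actors filtered by each entry, passing the first valid hit back to the unit through OverlapFromAgressiveComponent.
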(event `UpdateTargetActor`
  (bind _asbp_tracing_unit (cast `/Game/GameObject/Unit/BP_TracingUnit` (`self.GetOwner`))
    (:`then`
      (set `self.OwnerTargetActorArray` (`/Game/GameObject/Unit/BP_TracingUnit.TargetActorArray` _asbp_tracing_unit)))
    (:`CastFailed`
      (`self.K2_DestroyComponent`))))

(event `self.ReceiveBeginPlay`
  (`|ExecutionSequence`
    (:`then_0`
      (`self.UpdateTargetActor`))))

(event `self.ReceiveTick`
  (params (DeltaSeconds :type "Float (single-precision)"))
  (`self.CollisionProcess`))

(event `CollisionProcess`
  (for _array_element (`self.OwnerTargetActorArray`)
    (bind _item (`KismetArrayLibrary.Array_Get` (`Actor.GetOverlappingActors` (`self.GetOwner`) _array_element)))
    (`/Engine/EditorBlueprintResources/StandardMacros.IsValid` _item
      (:`Is Valid`
        (`self.Overlap` _item)
        (break)))))

(event `Overlap`
  (params (NewParam :type "Actor Object Reference"))
  (bind _asbp_tracing_unit (cast `/Game/GameObject/Unit/BP_TracingUnit` (`self.GetOwner`)))
  (`/Game/GameObject/Unit/BP_TracingUnit.OverlapFromAgressiveComponent` _asbp_tracing_unit NewParam))