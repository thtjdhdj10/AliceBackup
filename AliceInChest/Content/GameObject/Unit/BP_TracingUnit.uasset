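; BP_TracingUnit is a unit that is lured toward the nearest perceptible target.
; Perception updates keep actors of listed classes whose BP_BePerceptibleComponent allows perception, then select the closest.
; Tick starts a delayed SimpleMoveToActor when the unit is nearly stationary and uses a gate to stop it once the target is invalid.
; The construction script places a perception cone; priority and distance-limit logic is left disconnected.
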(event `self.ReceiveTick`
  (params (DeltaSeconds :type "Float (single-precision)"))
  (`|ExecutionSequence`
    (:`then_0`
      (`self.TraceProcess`))
    (:`then_1`
      (set `CharacterMovementComponent.MaxWalkSpeed` (`self.WalkSpeed`) (`self.CharacterMovement`)))))

(event `self.AIPerception.OnPerceptionUpdated`
  (params (UpdatedActors :type "Array of Actor Object Reference"))
  (`KismetArrayLibrary.Array_Clear` (`self.CorrectTargetArray`))
  (for _array_element UpdatedActors
    (bind _newparam1 (`self.CheckPerceptingActorIsValid` _array_element))
    (if _newparam1
      (`KismetArrayLibrary.Array_Add` (`self.CorrectTargetArray`) _array_element)))
  (`self.GetNearestInArray` (`self.CorrectTargetArray`)))

(event `TraceProcess`
  ;[1 1 1] be Lured to Target( TODO: using beHavier tree)
  (`|ExecutionSequence`
    (:`then_0`
      (`/Engine/EditorBlueprintResources/StandardMacros.Gate` true :!label _label
        (:`Exit`
          (`/Engine/EditorBlueprintResources/StandardMacros.IsValid` (`self.NearestTarget`)
            (:`Is Not Valid`
              (`self.StopTrace`)
              (goto _label :!via `Close`))))))
    (:`then_1`
      (if (`KismetMathLibrary.NearlyEqual_FloatFloat` (`KismetMathLibrary.VSizeSquared` (`MovementComponent.Velocity` (`self.CharacterMovement`))) 0.0 0.1)
        (`/Engine/EditorBlueprintResources/StandardMacros.IsValid` (`self.NearestTarget`)
          (:`Is Valid`
            (`self.StartTrace`)
            (goto _label :!via `Open`)))))))

(event `StartTrace`
  (`KismetSystemLibrary.Delay` (`self.TraceStartdelay`))
  (`NavigationSystem.SimpleMoveToActor` (`self.GetController`) (`self.NearestTarget`)))

(event `StopTrace`
  (`MovementComponent.StopMovementImmediately` (`self.CharacterMovement`)))

(event `OverlapFromAgressiveComponent`
  (params (NewParam :type "Actor Object Reference")))

(fn `CheckPerceptingActorIsValid`
  (params (NewParam :type "Actor Object Reference"))
  (returns (NewParam1 :type Boolean))
  (bind _returnvalue (`self.GetComponentByClass` NewParam "/Game/GameObject/Unit/BP_BePerceptibleComponent.BP_BePerceptibleComponent_C"))
  (for _array_element (`self.TargetActorArray`)
    (if (== _array_element (`GameplayStatics.GetObjectClass` NewParam))
      (`/Engine/EditorBlueprintResources/StandardMacros.IsValid` _returnvalue
        (:`Is Valid`
          (if (`/Game/GameObject/Unit/BP_BePerceptibleComponent.bCanBePercepted` _returnvalue)
            (return true)
            (else
              _)))
        (:`Is Not Valid`
          _))
      (return false))))

(fn `GetNearestInArray`
  (params (NewParam :type "Array of Actor Object Reference"))
  (set `self.NearestPriorityDistance` 9999999999.0)
  (if (== 0 (`KismetArrayLibrary.Array_Length` NewParam))
    (set `self.NearestTarget` null)
    (else
      (for _array_element NewParam
        (bind _returnvalue (`self.GetDistanceTo` _array_element))
        (if (< _returnvalue (`self.NearestPriorityDistance`))
          (set `self.NearestTarget` _array_element)
          (set `self.NearestPriorityDistance` _returnvalue))))))

(fn `UserConstructionScript`
  (bind _perceptiondisplaycone (`self.PerceptionDisplayCone`))
  (`SceneComponent.SetWorldScale3D` _perceptiondisplaycone (1.8 2.0 1.8))
  (`SceneComponent.K2_SetRelativeLocation` _perceptiondisplaycone (`KismetMathLibrary.MakeVector` (* (* (`self.PerceptionVolumePositionRatio`) (.x (`SceneComponent.RelativeScale3D` (`self.PerceptionDisplayCone`)))) 1.0) 0.0 (* (`CapsuleComponent.GetScaledCapsuleHalfHeight` (`self.CapsuleComponent`)) 0.5)) false false))