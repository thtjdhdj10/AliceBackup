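; BP_Spider is an enemy unit that restarts the current level when it catches Alice.
; It overrides the parent's aggressive-component overlap event, calling the parent logic first.
; If the overlapping object's class is exactly BP_Alice, it fetches the current level name and reopens that level.
; Tick is disabled, and construction only defers to the parent.
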(event `self.OverlapFromAgressiveComponent`
  (params (NewParam :type "Actor Object Reference"))
  (`parent.OverlapFromAgressiveComponent` NewParam)
  (if (== (`GameplayStatics.GetObjectClass` NewParam) "/Game/GameObject/Unit/BP_Alice.BP_Alice_C")
    (bind _returnvalue (`GameplayStatics.GetCurrentLevelName` true))
    (`GameplayStatics.OpenLevel` (`KismetStringLibrary.Conv_StringToName` _returnvalue))))

(fn `UserConstructionScript`
  (`parent.UserConstructionScript`))