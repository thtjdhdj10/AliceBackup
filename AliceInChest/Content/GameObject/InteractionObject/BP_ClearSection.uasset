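; BP_ClearSection is an interactable level exit that lets Alice move on to the next level once it is open.
; Every tick, the Cube's material switches between open and closed looks based on the BPConditionalComponent's Opened flag.
; When BP_Alice begins overlapping the Cube while it is open, a DoOnce guard loads the level named by NextLevelName.
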(event `self.ReceiveTick`
  (params (DeltaSeconds :type "Float (single-precision)"))
  (if (`/Game/GameObject/InteractionObject/BP_ConditionalComponent.bOpened` (`self.BP_ConditionalComponent`))
    (`PrimitiveComponent.SetMaterial` (`self.Cube`) 0 "/Game/Materials/M_OpenedSection.M_OpenedSection")
    (else
      (`PrimitiveComponent.SetMaterial` (`self.Cube`) 0 "/Game/Materials/M_ClosedSection.M_ClosedSection"))))

(event `self.Cube.OnComponentBeginOverlap`
  (params (OverlappedComponent :type "PrimitiveComponent Object Reference") (OtherActor :type "Actor Object Reference") (OtherComp :type "PrimitiveComponent Object Reference") (OtherBodyIndex :type Integer) (bFromSweep :type Boolean) (SweepResult :type "HitResult Structure (by ref)"))
  (if (`/Game/GameObject/InteractionObject/BP_ConditionalComponent.bOpened` (`self.BP_ConditionalComponent`))
    (if (== (`GameplayStatics.GetObjectClass` OtherActor) "/Game/GameObject/Unit/BP_Alice.BP_Alice_C")
      (`/Engine/EditorBlueprintResources/StandardMacros.DoOnce` false
        (:`Completed`
          (`GameplayStatics.OpenLevel` (`self.NextLevelName`)))))))

(fn `UserConstructionScript`
  (`parent.UserConstructionScript`))