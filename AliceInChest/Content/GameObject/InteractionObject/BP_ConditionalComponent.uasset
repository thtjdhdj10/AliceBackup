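; BP_ConditionalComponent is an interaction-object component that reports an Opened state based on the trigger actors listed in TriggerForOpen.
; BeginPlay opens it when the list is empty and prunes invalid entries in reverse order.
; Tick polls each actor's BP_TriggerComponent, clearing Opened if any is inactive, so actors without that component never block it.
; An OnRep_bOpened handler exists but is empty.
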(event `self.ReceiveBeginPlay`
  (bind _triggerforopen (`self.TriggerForOpen`))
  (bind _returnvalue (`KismetArrayLibrary.Array_Length` (`self.TriggerForOpen`)))
  (bind _returnvalue_2 (> _returnvalue 0))
  (set `self.bOpened` (not _returnvalue_2))
  (if _returnvalue_2
    (for _index (range (- _returnvalue 1) 1)
      (`/Engine/EditorBlueprintResources/StandardMacros.IsValid` (`KismetArrayLibrary.Array_Get` _triggerforopen _index)
        (:`Is Not Valid`
          (`KismetArrayLibrary.Array_Remove` _triggerforopen _index))))))

(event `self.ReceiveTick`
  (params (DeltaSeconds :type "Float (single-precision)"))
  (set `self.bOpened` true)
  (for _array_element (`self.TriggerForOpen`)
    (`/Engine/EditorBlueprintResources/StandardMacros.IsValid` _array_element
      (:`Is Valid`
        (bind _returnvalue (`Actor.GetComponentByClass` _array_element "/Game/GameObject/InteractionObject/BP_TriggerComponent.BP_TriggerComponent_C"))
        (`/Engine/EditorBlueprintResources/StandardMacros.IsValid` _returnvalue
          (:`Is Valid`
            (if (not (`/Game/GameObject/InteractionObject/BP_TriggerComponent.bActive` _returnvalue))
              (set `self.bOpened` false)
              (break))))))))

(fn `OnRep_bOpened`)