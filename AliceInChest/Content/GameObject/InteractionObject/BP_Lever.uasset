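; BP_Lever is a one-shot interaction lever that activates its BPTriggerComponent when pressed.
; A Box overlap with a valid actor runs through a DoOnce fed by a BP_Alice class check, then calls Pressed.
; Pressed sets the trigger component active and swaps the Cube material to M_OpenedObject as visual feedback, with no path to reset it.
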(event `Pressed`
  (set `/Game/GameObject/InteractionObject/BP_TriggerComponent.bActive` true (`self.BP_TriggerComponent`))
  (`PrimitiveComponent.SetMaterial` (`self.Cube`) 0 "/Game/Materials/M_OpenedObject.M_OpenedObject"))

(event `self.Box.OnComponentBeginOverlap`
  (params (OverlappedComponent :type "PrimitiveComponent Object Reference") (OtherActor :type "Actor Object Reference") (OtherComp :type "PrimitiveComponent Object Reference") (OtherBodyIndex :type Integer) (bFromSweep :type Boolean) (SweepResult :type "HitResult Structure (by ref)"))
  (`/Engine/EditorBlueprintResources/StandardMacros.IsValid` OtherActor
    (:`Is Valid`
      (`/Engine/EditorBlueprintResources/StandardMacros.DoOnce` (== (`GameplayStatics.GetObjectClass` OtherActor) "/Game/GameObject/Unit/BP_Alice.BP_Alice_C")
        (:`Completed`
          (`self.Pressed`))))))

(fn `UserConstructionScript`
  (`parent.UserConstructionScript`))