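; BP_PressingTile is a pressure-plate interaction object that actors with a BP_PressableComponent can press by standing on it.
; Box overlaps from such actors raise and lower OverlapCounter, so the tile releases only when the last one leaves.
; Pressed and Released toggle BPTriggerComponent's Active flag and swap the Cube material between the opened and closed looks.
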(event `Pressed`
  (set `/Game/GameObject/InteractionObject/BP_TriggerComponent.bActive` true (`self.BP_TriggerComponent`))
  (`PrimitiveComponent.SetMaterial` (`self.Cube`) 0 "/Game/Materials/M_OpenedObject.M_OpenedObject"))

(event `Released`
  (set `/Game/GameObject/InteractionObject/BP_TriggerComponent.bActive` false (`self.BP_TriggerComponent`))
  (`PrimitiveComponent.SetMaterial` (`self.Cube`) 0 "/Game/Materials/M_ClosedObject.M_ClosedObject"))

(event `self.Box.OnComponentBeginOverlap`
  (params (OverlappedComponent :type "PrimitiveComponent Object Reference") (OtherActor :type "Actor Object Reference") (OtherComp :type "PrimitiveComponent Object Reference") (OtherBodyIndex :type Integer) (bFromSweep :type Boolean) (SweepResult :type "HitResult Structure (by ref)"))
  (`/Engine/EditorBlueprintResources/StandardMacros.IsValid` (`self.GetComponentByClass` OtherActor "/Game/GameObject/Unit/BP_PressableComponent.BP_PressableComponent_C")
    (:`Is Valid`
      (`/Engine/EditorBlueprintResources/StandardMacros.IncrementInt` (`self.OverlapCounter`)
        (:`  `
          (`self.Pressed`))))))

(event `self.Box.OnComponentEndOverlap`
  (params (OverlappedComponent :type "PrimitiveComponent Object Reference") (OtherActor :type "Actor Object Reference") (OtherComp :type "PrimitiveComponent Object Reference") (OtherBodyIndex :type Integer))
  (bind _overlapcounter (`self.OverlapCounter`))
  (`/Engine/EditorBlueprintResources/StandardMacros.IsValid` (`self.GetComponentByClass` OtherActor "/Game/GameObject/Unit/BP_PressableComponent.BP_PressableComponent_C")
    (:`Is Valid`
      (`/Engine/EditorBlueprintResources/StandardMacros.DecrementInt` _overlapcounter
        (:`  `
          (if (<= _overlapcounter 0)
            (`self.Released`)))))))

(fn `UserConstructionScript`
  (`parent.UserConstructionScript`))