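; BP_ChestGround is a static arena object that builds a ground enclosed by four walls and fits a navigation mesh actor to it.
; The construction script derives the NavMesh scale and all wall transforms from the Ground's world scale, using shared box size, wall thickness and wall height values.
; Each wall has its own placement function, with front and back rotated 90 degrees.
; Positions are absolute world coordinates centered on the origin, independent of the actor's location.
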(fn `UserConstructionScript`
  (bind _navmesh (`self.NavMesh`))
  (bind _returnvalue (`SceneComponent.K2_GetComponentScale` (`self.Ground`)))
  (`self.SetActorScale3D` _navmesh (* _returnvalue (0.5 0.5 10.0)))
  (`self.K2_SetActorLocation` _navmesh (`KismetMathLibrary.MakeVector` 0.0 0.0 (* 10.0 10.0)) false false)
  (set `self.xScale` (.x _returnvalue))
  (set `self.yScale` (.y _returnvalue))
  (`|ExecutionSequence`
    (:`then_0`
      (`self.LeftWallTransformSet`))
    (:`then_1`
      (`self.RightWallTransformSet`))
    (:`then_2`
      (`self.FrontWallTransformSet`))
    (:`then_3`
      (`self.BackWallTransformSet`))))